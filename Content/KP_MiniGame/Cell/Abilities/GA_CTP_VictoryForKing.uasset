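; Cell gameplay ability for the KP minigame that declares a reach-the-point victory, named as the King's win condition.
; On activation it commits, casts the triggering event's target to a BoardPiece and compares its player ID to the owning player ID from GetInfo.
; If they differ, it adds the non-replicated WinCondition.ReachThePoint loose tag to the GameMode and prints "Victory".
; It contains no check that the piece is a King.
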(event `self.K2_ActivateAbility`
  (bind (_returnvalue_abilityclass _returnvalue_owningplayerid) (break `GameplayAbilityCellToPawnInfo` (`self.GetInfo`)))
  (bind (_currenteventdata_eventtag _currenteventdata_instigator _currenteventdata_target) (break `GameplayEventData` (`self.CurrentEventData`)))
  (bind _returnvalue (`self.K2_CommitAbility`))
  (if _returnvalue
    (bind _asboard_piece (cast `BoardPiece` _currenteventdata_target)
      (:`then`
        (if (== _returnvalue_owningplayerid (`BoardPiece.OwnPlayerId` _asboard_piece))
          (`self.K2_EndAbility`)
          (else
            (`AbilitySystemBlueprintLibrary.AddLooseGameplayTags` (`GameplayStatics.GetGameMode`) (`BlueprintGameplayTagLibrary.MakeGameplayTagContainerFromArray` (`|MakeArray` (struct :`TagName` "WinCondition.ReachThePoint") :!type "GameplayTag Structure")))
            (`KismetSystemLibrary.PrintString` "Victory")
            (`self.K2_EndAbility`))))
      (:`CastFailed`
        (`self.K2_EndAbility`)))
    (else
      (`self.K2_EndAbility`))))