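; Gameplay ability in the KP minigame's cell ability set that requests an upgrade for a targeted Pawn board piece.
; It responds only to gameplay events whose target is a BoardPiece of type Pawn.
; On activation it forwards that target to KP_GameMode in a GameplayEvent.BoardPiece.UpgradePawn event and ends, leaving the upgrade itself to the receiver.
; If the game mode cast fails, it cancels.
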(event `self.K2_ActivateAbility`
  (bind (_currenteventdata_eventtag _currenteventdata_instigator _currenteventdata_target) (break `GameplayEventData` (`self.CurrentEventData`)))
  (bind _askp_game_mode (cast `/Game/KP_MiniGame/Blueprints/KP_GameMode` (`GameplayStatics.GetGameMode`))
    (:`then`
      (`AbilitySystemBlueprintLibrary.SendGameplayEventToActor` _askp_game_mode (struct :`TagName` "GameplayEvent.BoardPiece.UpgradePawn") (make `GameplayEventData` (struct :`TagName` "GameplayEvent.BoardPiece.UpgradePawn") null _currenteventdata_target))
      (`self.K2_EndAbility`))
    (:`CastFailed`
      (`self.K2_CancelAbility`))))

(fn `K2_ShouldAbilityRespondToEvent`
  (params (ActorInfo :type "GameplayAbilityActorInfo Structure") (Payload :type "GameplayEventData Structure"))
  (returns (ReturnValue :type Boolean))
  (bind _asboard_piece (cast `BoardPiece` (`.Target` (break `GameplayEventData` Payload)))
    (:`then`
      (return (`|EnumEquality` (`BoardPiece.GetBoardPieceType` _asboard_piece) "Pawn")))
    (:`CastFailed`
      (return false))))