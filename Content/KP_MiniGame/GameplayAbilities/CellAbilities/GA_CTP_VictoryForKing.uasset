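; GA_CTP_VictoryForKing is a board-cell gameplay ability that awards a reach-the-point victory.
; On activation it commits, casts the event's target to a BoardPiece, and checks that the piece is a Pawn whose owner matches the ability info's owning player.
; A match adds the WinCondition.ReachThePoint loose tag to the GameMode, prints a debug message and ends.
; Any failure cancels the ability.
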(event `self.K2_ActivateAbility`
  (bind (_returnvalue_data _returnvalue_owningplayerid) (break `GameplayAbilityCellToPawnInfo` (`self.GetInfo`)))
  (bind (_currenteventdata_eventtag _currenteventdata_instigator _currenteventdata_target) (break `GameplayEventData` (`self.CurrentEventData`)))
  (bind _returnvalue (`self.K2_CommitAbility`))
  (if _returnvalue
    (bind _asboard_piece (cast `BoardPiece` _currenteventdata_target)
      (:`then`
        (if (and (== _returnvalue_owningplayerid (`BoardPiece.OwnPlayerId` _asboard_piece)) (`|EnumEquality` (`BoardPiece.GetBoardPieceType` _asboard_piece) "Pawn"))
          (`AbilitySystemBlueprintLibrary.AddLooseGameplayTags` (`GameplayStatics.GetGameMode`) (`BlueprintGameplayTagLibrary.MakeGameplayTagContainerFromArray` (`|MakeArray` (struct :`TagName` "WinCondition.ReachThePoint") :!type "GameplayTag Structure")))
          (`KismetSystemLibrary.PrintString` "Victory")
          (`self.K2_EndAbility`)
          (else
            (`self.K2_CancelAbility`))))
      (:`CastFailed`
        (`self.K2_CancelAbility` :!label _label)))
    (else
      (goto _label))))