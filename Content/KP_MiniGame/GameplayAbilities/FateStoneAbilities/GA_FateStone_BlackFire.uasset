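; Fate Stone gameplay ability for the KP minigame that puts the BlackFire effect on a targeted Cell.
; On activation it reads the target from the event data, has that Cell's AbilitySystemComponent apply GE_CellEffect_BlackFire to itself, then ends.
; A non-Cell target cancels the ability.
; CanUseFateStone allows only Cell targets that also pass the parent's check.
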(event `self.K2_ActivateAbility`
  (bind (_currenteventdata_eventtag _currenteventdata_instigator _currenteventdata_target) (break `GameplayEventData` (`self.CurrentEventData`)))
  (`parent.K2_ActivateAbility`)
  (bind _ascell (cast `Cell` _currenteventdata_target)
    (:`then`
      (bind _abilitysystemcomponent (`Cell.AbilitySystemComponent` _ascell))
      (`AbilitySystemComponent.BP_ApplyGameplayEffectSpecToTarget` _abilitysystemcomponent (`self.MakeOutgoingGameplayEffectSpec` "/Game/KP_MiniGame/GameplayAbilities/FateStoneEffects/CellEffects/GE_CellEffect_BlackFire.GE_CellEffect_BlackFire_C") _abilitysystemcomponent)
      (`self.K2_EndAbility`))
    (:`CastFailed`
      (`self.K2_CancelAbility`))))

(fn `CanUseFateStone`
  (params (Target :type "Actor Object Reference") (Owner :type "Actor Object Reference") (FateStoneActions :type Integer))
  (returns (ReturnValue :type Boolean))
  (cast `Cell` Target
    (:`then`
      (return (and true (`parent.CanUseFateStone` Target Owner FateStoneActions))))
    (:`CastFailed`
      (return false))))