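; Cold Mist Fate Stone ability for the board mini-game that applies the GE_ColdMist gameplay effect to a targeted board piece.
; On activation it takes the piece from the event data's Target, applies the effect through that piece's own ability system component and ends, or cancels if the target is not a BoardPiece.
; CanUseFateStone adds a BoardPiece type check to the parent's usability rules.
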(event `self.K2_ActivateAbility`
  (bind (_currenteventdata_eventtag _currenteventdata_instigator _currenteventdata_target) (break `GameplayEventData` (`self.CurrentEventData`)))
  (`parent.K2_ActivateAbility`)
  (bind _asboard_piece (cast `BoardPiece` _currenteventdata_target)
    (:`then`
      (bind _abilitysystemcomponent (`BoardPiece.AbilitySystemComponent` _asboard_piece))
      (`AbilitySystemComponent.BP_ApplyGameplayEffectSpecToTarget` _abilitysystemcomponent (`self.MakeOutgoingGameplayEffectSpec` "/Game/KP_MiniGame/GameplayAbilities/FateStoneEffects/BoardPieceEffects/GE_ColdMist.GE_ColdMist_C") _abilitysystemcomponent)
      (`self.K2_EndAbility`))
    (:`CastFailed`
      (`self.K2_CancelAbility`))))

(fn `CanUseFateStone`
  (params (Target :type "Actor Object Reference") (Owner :type "Actor Object Reference") (FateStoneActions :type Integer))
  (returns (ReturnValue :type Boolean))
  (return (and (`GameplayStatics.ObjectIsA` Target "/Script/KP_Minigame.BoardPiece") (`parent.CanUseFateStone` Target Owner FateStoneActions))))