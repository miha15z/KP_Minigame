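; GA_FateStone_FlamingArrow is a Fate Stone gameplay ability that instantly kills an opposing board piece in the KP minigame.
; On activation it reads instigator and target from the event data, force-kills an enemy King and ends, otherwise cancels.
; CanUseFateStone requires remaining Fate Stone actions and an enemy Pawn target, so its piece-type check differs from the King check used on activation.
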(event `self.K2_ActivateAbility`
  (bind (_currenteventdata_eventtag _currenteventdata_instigator _currenteventdata_target) (break `GameplayEventData` (`self.CurrentEventData`)))
  (`parent.K2_ActivateAbility`)
  (bind _askppawn (cast `KPPawn` _currenteventdata_instigator)
    (:`then`
      (bind _asboard_piece (cast `BoardPiece` _currenteventdata_target)
        (:`then`
          (if (and (`|EnumEquality` (`BoardPiece.GetBoardPieceType` _asboard_piece) "King") (!= (`BoardPiece.OwnPlayerId` _asboard_piece) (`KPPawn.PlayerId` _askppawn)))
            (`BoardPiece.ForceKill` _asboard_piece)
            (`self.K2_EndAbility`)
            (else
              (`self.K2_CancelAbility`))))
        (:`CastFailed`
          (`self.K2_CancelAbility` :!label _label))))
    (:`CastFailed`
      (goto _label))))

(fn `CanUseFateStone`
  (params (Target :type "Actor Object Reference") (Owner :type "Actor Object Reference") (FateStoneActions :type Integer))
  (returns (ReturnValue :type Boolean))
  (`|ExecutionSequence`
    (:`then_0`
      (if (not (> FateStoneActions 0))
        (return false)))
    (:`then_1`
      (bind _asboard_piece (cast `BoardPiece` Target)
        (:`then`
          (bind _askppawn (cast `KPPawn` Owner)
            (:`then`
              (if (and (`|EnumEquality` (`BoardPiece.GetBoardPieceType` _asboard_piece) "Pawn") (!= (`BoardPiece.OwnPlayerId` _asboard_piece) (`KPPawn.PlayerId` _askppawn)))
                (return true)
                (else
                  (return false))))
            (:`CastFailed`
              (return false))))
        (:`CastFailed`
          (return false))))))